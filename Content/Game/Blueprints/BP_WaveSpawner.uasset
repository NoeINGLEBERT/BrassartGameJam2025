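; BP_WaveSpawner is a wave spawner that spawns planet actors from an enemy pool at random points in a distant shell around the world origin.
; On BeginPlay it starts the current wave, updating the GameInstance, playing the HUD animation and loading the BT_WaveSysteme row's class-to-count map.
; Tick, throttled by a Delay, spawns one planet per pass and decrements its count.
; A separate queue spawns planets at the spawner's transform on a timer.
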(event Custom|StartWave
  (bind _player (Variables|Default|GetPlayer))
  (bind _hud (Variables|/Game/Game/Blueprints/BP_Player.BP_Player_C|GetHUD _player))
  (Variables|/Game/Game/Blueprints/GI_Game.GI_Game_C|SetWave (Variables|Default|GetGameInstance) (Variables|Default|GetWave%20Number))
  (Class|UserWidget|PlayAnimationForward _hud (Variables|/Game/Game/Widget/WBP_HUD.WBP_HUD_C|GetWaveChange _hud) 1.0 false)
  (bind _outrownames (DataTable|GetDataTableRowNames "/Game/Datatables/BT_WaveSysteme.BT_WaveSysteme"))
  (bind _returnvalue (Utilities|GetDataTableRow "/Game/Datatables/BT_WaveSysteme.BT_WaveSysteme" (Utilities|Array|Get(acopy) _outrownames (Variables|Default|GetWave%20Number)))
    (:then
      (Variables|Default|SetCurrentRowPool (.enemypool _returnvalue)))))

(event EventBeginPlay
  (bind _returnvalue (Actor|GetActorOfClass "/Game/Game/Blueprints/BP_Player.BP_Player_C"))
  (Variables|Default|SetPlayer _returnvalue)
  (bind _asgi_game (Utilities|Casting|CastToGI_Game (Game|GetGameInstance)))
  (Variables|Default|SetGameInstance _asgi_game)
  (CallFunction|StartWave))

(event EventTick
  (params (DeltaSeconds :type Float%20%28single-precision%29))
  (bind _currentrowpool (Variables|Default|GetCurrentRowPool))
  (Utilities|FlowControl|Delay 1.0)
  (bind _keys (Utilities|Map|Keys _currentrowpool))
  (bind _values (Utilities|Map|Values _currentrowpool))
  (bind (_array_element _array_index) (Utilities|Array|ForEachLoopwithBreak _values :!label _label)
    (:LoopBody
      (if (!= _array_element 0)
        (Variables|Default|SetTempValue (- _array_element 1))
        (CallFunction|SpawnPlanetfromClass (Utilities|Array|Get(acopy) _keys _array_index))
        (Utilities|Map|Remove _currentrowpool (Utilities|Array|Get(acopy) _keys _array_index))
        (Utilities|Map|Add (Variables|Default|GetCurrentRowPool) (Utilities|Array|Get(acopy) _keys _array_index) (Variables|Default|GetTempValue))
        (goto _label Break)))))

(fn ConstructionScript)

(fn SpawnPlanet
  (if (Utilities|Array|IsValidIndex (Variables|Default|GetPlanetQueue))
    (Game|SpawnActorfromClass (Utilities|Array|Get(acopy) (Variables|Default|GetPlanetQueue)) (Transformation|GetActorTransform) "Undefined" "MultiplyWithRoot" 0 0)
    (Utilities|Array|RemoveIndex (Variables|Default|GetPlanetQueue))
    (Utilities|Time|SetTimerbyFunctionName 0 "SpawnPlanet" 1e+01)
    (return true)
    (else
      (return false))))

(fn AddPlanettoQueue
  (params (NewItem :type BP%20Enemy%20Planet%20Class%20Reference%20%28by%20ref%29))
  (Utilities|Array|Add (Variables|Default|GetPlanetQueue) NewItem)
  (CallFunction|SpawnPlanet))

(fn SpawnPlanetfromClass
  (params (Class :type Actor%20Class%20Reference))
  (Game|SpawnActorfromClass Class (Math|Transform|MakeTransform (* (Math|Random|RandomUnitVector) (Math|Random|RandomFloatinRange 2e+06 3e+06)) (Math|Random|RandomRotator true) "1.000000,1.000000,1.000000") "Undefined" "MultiplyWithRoot" 0 0))