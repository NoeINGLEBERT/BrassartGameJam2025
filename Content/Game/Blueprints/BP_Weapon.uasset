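; BP_Weapon is a weapon that fires projectiles toward the player's calculated target point with slight random cone spread.
; Shoot input runs gates that pace shots by charge delay and RPM, with a per-tick retry loop.
; Each shot spends ammo, spawns the configurable projectile and plays a Niagara muzzle flash; ChargeVFX is an empty hook.
; An empty magazine or reload input triggers a DoOnce-guarded timed reload, re-armed when firing with ammo.
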(event Custom|IA_Shoot%20%28Triggered%29
  (if (== (Variables|Default|GetCurrentAmmo) 0)
    (Utilities|FlowControl|Sequence
      (:then_0
        (Utilities|FlowControl|Gate true) ; enters at Close
      )
      (:then_1
        (Utilities|FlowControl|DoOnce false :!label _label
          (:Completed
            (CallFunction|Reload)))))
    (else
      (Utilities|FlowControl|Sequence
        (:then_0
          (goto _label Reset))
        (:then_1
          (Utilities|FlowControl|Gate false :!label _label_2
            (:Exit
              (Utilities|FlowControl|Sequence
                (:then_0
                  (goto _label_2 Close))
                (:then_1
                  (Utilities|FlowControl|Sequence
                    (:then_0
                      (CallFunction|ChargeVFX))
                    (:then_1
                      (Utilities|FlowControl|Delay (Variables|Default|GetChargeDelay))
                      (Utilities|FlowControl|Sequence
                        (:then_0
                          (Math|Integer|DecrementInt (Variables|Default|GetCurrentAmmo)
                            (:%20%20
                              (Utilities|FlowControl|Sequence
                                (:then_0
                                  (bind _returnvalue (Game|SpawnActorfromClass (Variables|Default|GetProjectileClass) (Math|Transform|MakeTransform (Transformation|GetWorldLocation (Variables|Default|GetProjectileSpawnPoint)) (Math|Rotator|MakeRotfromXZ (Math|Random|RandomUnitVectorinConeinDegrees (- (Default|CalculateTargetPoint (Variables|Default|GetPlayer)) (Transformation|GetActorLocation)) 1.0) (Math|Vector|MakeVector 0.0 0.0 1.0)) "5.000000,5.000000,5.000000") "Undefined" "MultiplyWithRoot" 0 0))
                                  (Default|BeginPlay _returnvalue self (Variables|Default|GetDamage)))
                                (:then_1
                                  (CallFunction|MuzzleFlash (Transformation|GetWorldTransform (Variables|Default|GetProjectileSpawnPoint))))))))
                        (:then_1
                          (Utilities|FlowControl|Delay (/ 6e+01 (Variables|Default|GetRPM)))
                          (goto _label_2 Open))
                        (:then_2
                          (Utilities|FlowControl|Gate true) ; enters at Toggle
                        )))))))))))))

(event Custom|IA_Shoot%20%28Started%29
  (Utilities|FlowControl|Sequence
    (:then_0
      (goto _label Open))
    (:then_1
      (Utilities|FlowControl|Gate true :!label _label
        (:Exit
          (Utilities|FlowControl|Sequence
            (:then_0
              (if (== (Variables|Default|GetCurrentAmmo) 0)
                (Utilities|FlowControl|Sequence
                  (:then_0
                    (goto _label Close))
                  (:then_1
                    (Utilities|FlowControl|DoOnce false :!label _label_2
                      (:Completed
                        (CallFunction|Reload)))))
                (else
                  (Utilities|FlowControl|Sequence
                    (:then_0
                      (goto _label_2 Reset))
                    (:then_1
                      (Utilities|FlowControl|Gate false :!label _label_3
                        (:Exit
                          (Utilities|FlowControl|Sequence
                            (:then_0
                              (goto _label_3 Close))
                            (:then_1
                              (Utilities|FlowControl|Sequence
                                (:then_0
                                  (CallFunction|ChargeVFX))
                                (:then_1
                                  (Utilities|FlowControl|Delay (Variables|Default|GetChargeDelay))
                                  (Utilities|FlowControl|Sequence
                                    (:then_0
                                      (Math|Integer|DecrementInt (Variables|Default|GetCurrentAmmo)
                                        (:%20%20
                                          (Utilities|FlowControl|Sequence
                                            (:then_0
                                              (bind _returnvalue (Game|SpawnActorfromClass (Variables|Default|GetProjectileClass) (Math|Transform|MakeTransform (Transformation|GetWorldLocation (Variables|Default|GetProjectileSpawnPoint)) (Math|Rotator|MakeRotfromXZ (Math|Random|RandomUnitVectorinConeinDegrees (- (Default|CalculateTargetPoint (Variables|Default|GetPlayer)) (Transformation|GetActorLocation)) 1.0) (Math|Vector|MakeVector 0.0 0.0 1.0)) "5.000000,5.000000,5.000000") "Undefined" "MultiplyWithRoot" 0 0))
                                              (Default|BeginPlay _returnvalue self (Variables|Default|GetDamage)))
                                            (:then_1
                                              (CallFunction|MuzzleFlash (Transformation|GetWorldTransform (Variables|Default|GetProjectileSpawnPoint))))))))
                                    (:then_1
                                      (Utilities|FlowControl|Delay (/ 6e+01 (Variables|Default|GetRPM)))
                                      (goto _label_3 Open))
                                    (:then_2
                                      (goto _label Toggle))))))))))))))
            (:then_1
              (Utilities|FlowControl|Delay 0.0)
              (goto _label))))))))

(event Custom|MuzzleFlash
  (params (Transform :type Transform))
  (Niagara|SpawnSystematLocation "/Game/Game/VFX/NS_MuzzleFlash.NS_MuzzleFlash" (.location Transform) (.rotation Transform)))

(event Custom|ChargeVFX)

(event Custom|Reload
  (Development|PrintString "Reload Start")
  (Variables|Default|SetReloadStartTime (Utilities|Time|GetTimeSeconds))
  (Variables|Default|SetCurrentAmmo 0)
  (Utilities|FlowControl|Delay (Variables|Default|GetReloadTime))
  (Variables|Default|SetCurrentAmmo (Variables|Default|GetMaxAmmo))
  (Development|PrintString "Reload End"))

(event Custom|IA_Reload
  (Utilities|FlowControl|DoOnce false
    (:Completed
      (CallFunction|Reload))))

(event EventBeginPlay
  (Variables|Default|SetCurrentAmmo (Variables|Default|GetMaxAmmo))
  (bind _returnvalue (Actor|GetActorOfClass "/Game/Game/Blueprints/BP_Player.BP_Player_C"))
  (Variables|Default|SetPlayer _returnvalue))

(fn ConstructionScript)