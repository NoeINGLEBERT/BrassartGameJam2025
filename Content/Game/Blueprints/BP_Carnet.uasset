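; BP_Carnet is a notebook-style weapon catalogue whose pages flip left or right to browse weapons to buy or equip.
; Four widget components show pages built from DT_WeaponWidgets, with French buy/equip labels from each weapon's state and cached page data.
; Turns shift the page indices, rebuild the widgets and play the PageTurn timeline forward or backward to swing the middle page.
; Gates block overlapping animations, and finishing re-syncs the visible pages.
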(event Custom|TurnLeft
  (bind _pageweaponindex (Variables|Default|GetPageWeaponIndex))
  (bind _pageweaponindex_2 (Variables|Default|GetPageWeaponIndex))
  (if (> (Utilities|Array|Get(acopy) (Variables|Default|GetPageWeaponIndex)) 0)
    (Audio|PlaySound2D "/Game/Game/SFX/UI/SC_Turn.SC_Turn" 1.0 1.0 0.0 0 0)
    (for _index (range 1 3)
      (Utilities|Array|SetArrayElem _pageweaponindex (- 3 _index) (- (Utilities|Array|Get(acopy) _pageweaponindex 3) _index)))
    (CallFunction|UpdateWidgets)
    (Utilities|FlowControl|Gate false :!label _label
      (:Exit
        (Utilities|FlowControl|Sequence
          (:then_0
            (goto _label Close))
          (:then_1
            (Utilities|FlowControl|Gate false) ; enters at Close
          )
          (:then_2
            (bind (_direction _alpha) (Timeline|Page%20Turn ReverseFromEnd)
              (:Update
                (Transformation|SetRelativeTransform (Variables|Default|GetMidPage) (Math|Transform|Lerp(Transform) (Transformation|GetRelativeTransform (Variables|Default|GetRightPage)) (Transformation|GetRelativeTransform (Variables|Default|GetLeftPage)) _alpha) false false)
                (Transformation|SetRelativeLocationAndRotation (Variables|Default|GetPlane) (Math|Vector|Lerp(Vector) "-4.570689,2.912544,0.000000" "-4.570689,-2.912544,0.000000" _alpha) (Math|Rotator|MakeRotator -9e+01 0.0 (Math|Float|Lerp 179.06301 360.93699 _alpha)) false false))
              (:Finished
                (Utilities|FlowControl|Sequence
                  (:then_0
                    (Utilities|FlowControl|Gate false) ; enters at Open
                  )
                  (:then_1
                    (goto _label Open))
                  (:then_2
                    (switch Utilities|FlowControl|Switch|SwitchonETimelineDirection _direction
                      (:Forward
                        (Utilities|Array|SetArrayElem _pageweaponindex_2 0 (Utilities|Array|Get(acopy) _pageweaponindex_2 2)))
                      (:Backward
                        (Utilities|Array|SetArrayElem _pageweaponindex_2 3 (Utilities|Array|Get(acopy) _pageweaponindex_2 1))))
                    (CallFunction|UpdateWidgets)))))))))))

(event Custom|TurnRight
  (bind _pageweaponindex (Variables|Default|GetPageWeaponIndex))
  (bind _pageweaponindex_2 (Variables|Default|GetPageWeaponIndex))
  (bind _outrownames (DataTable|GetDataTableRowNames "/Game/Datatables/DT_WeaponWidgets.DT_WeaponWidgets"))
  (if (< (+ (Utilities|Array|Get(acopy) (Variables|Default|GetPageWeaponIndex)) 3) (Utilities|Array|Length _outrownames))
    (Audio|PlaySound2D "/Game/Game/SFX/UI/SC_Turn.SC_Turn" 1.0 1.0 0.0 0 0)
    (for _index (range 1 3)
      (Utilities|Array|SetArrayElem _pageweaponindex _index (+ (Utilities|Array|Get(acopy) _pageweaponindex) _index)))
    (CallFunction|UpdateWidgets)
    (Utilities|FlowControl|Gate false :!label _label
      (:Exit
        (Utilities|FlowControl|Sequence
          (:then_0
            (goto _label Close))
          (:then_1
            (Utilities|FlowControl|Gate false) ; enters at Close
          )
          (:then_2
            (bind (_direction _alpha) (Timeline|Page%20Turn PlayFromStart)
              (:Update
                (Transformation|SetRelativeTransform (Variables|Default|GetMidPage) (Math|Transform|Lerp(Transform) (Transformation|GetRelativeTransform (Variables|Default|GetRightPage)) (Transformation|GetRelativeTransform (Variables|Default|GetLeftPage)) _alpha) false false)
                (Transformation|SetRelativeLocationAndRotation (Variables|Default|GetPlane) (Math|Vector|Lerp(Vector) "-4.570689,2.912544,0.000000" "-4.570689,-2.912544,0.000000" _alpha) (Math|Rotator|MakeRotator -9e+01 0.0 (Math|Float|Lerp 179.06301 360.93699 _alpha)) false false))
              (:Finished
                (Utilities|FlowControl|Sequence
                  (:then_0
                    (goto _label Open))
                  (:then_1
                    (Utilities|FlowControl|Gate false) ; enters at Open
                  )
                  (:then_2
                    (switch Utilities|FlowControl|Switch|SwitchonETimelineDirection _direction
                      (:Forward
                        (Utilities|Array|SetArrayElem _pageweaponindex_2 0 (Utilities|Array|Get(acopy) _pageweaponindex_2 2)))
                      (:Backward
                        (Utilities|Array|SetArrayElem _pageweaponindex_2 3 (Utilities|Array|Get(acopy) _pageweaponindex_2 1))))
                    (CallFunction|UpdateWidgets)))))))))))

(event EventBeginPlay
  (Variables|Default|SetPageWidgets (Utilities|Array|MakeArray (Variables|Default|GetLeftWidget) (Variables|Default|GetMidRightWidget) (Variables|Default|GetMidLeftWidget) (Variables|Default|GetRightWidget)))
  (CallFunction|UpdateWidgets))

(fn ConstructionScript)

(fn CreateWeaponWidget
  (params (WeaponIndex :type Integer))
  (bind _returnvalue (Math|Integer|%(Integer) WeaponIndex 2))
  (bind _states (Variables|Default|GetStates))
  (bind _output (Utilities|Array|Get(acopy) _states WeaponIndex))
  (bind _returnvalue_2 (== _returnvalue 0))
  (bind _outrownames (DataTable|GetDataTableRowNames "/Game/Datatables/DT_WeaponWidgets.DT_WeaponWidgets"))
  (bind _returnvalue_3 (Utilities|GetDataTableRow "/Game/Datatables/DT_WeaponWidgets.DT_WeaponWidgets" (Utilities|Array|Get(acopy) _outrownames WeaponIndex))
    (:then
      (Utilities|Array|Add (Variables|Default|GetPageClass) (.WeaponClass (Utilities|Struct|BreakWeaponWidgetStructure _returnvalue_3)))
      (bind _returnvalue_4 (UserInterface|CreateWidget "/Game/Game/Widget/WBP_WeaponParent.WBP_WeaponParent_C"))
      (Variables|Default|SetTempWidget _returnvalue_4)
      (Variables|/Script/UMG.TextBlock|SetText (Variables|/Game/Game/Widget/WBP_WeaponParent.WBP_WeaponParent_C|GetWeaponName _returnvalue_4) (.WeaponName (Utilities|Struct|BreakWeaponWidgetStructure _returnvalue_3)))
      (Appearance|SetBrushfromTexture (Variables|/Game/Game/Widget/WBP_WeaponParent.WBP_WeaponParent_C|GetWeaponImage _returnvalue_4) (.WeaponImage (Utilities|Struct|BreakWeaponWidgetStructure _returnvalue_3)))
      (Utilities|Array|Add (Variables|Default|GetPageTexture) (.WeaponImage (Utilities|Struct|BreakWeaponWidgetStructure _returnvalue_3)))
      (Variables|/Script/UMG.TextBlock|SetText (Variables|/Game/Game/Widget/WBP_WeaponParent.WBP_WeaponParent_C|GetWeaponDescription _returnvalue_4) (.WeaponDescription (Utilities|Struct|BreakWeaponWidgetStructure _returnvalue_3)))
      (Variables|/Script/UMG.TextBlock|SetText (Variables|/Game/Game/Widget/WBP_WeaponParent.WBP_WeaponParent_C|GetPageNumber _returnvalue_4) (Utilities|Text|ToText(Integer) (+ WeaponIndex 1)))
      (Class|Widget|SetRenderTranslation (Variables|/Game/Game/Widget/WBP_WeaponParent.WBP_WeaponParent_C|GetPageArrow _returnvalue_4) (select _returnvalue_2 "(X=-115.000000,Y=0.000000)" "(X=115.000000,Y=0.000000)"))
      (Widget|Transform|SetRenderScale (Variables|/Game/Game/Widget/WBP_WeaponParent.WBP_WeaponParent_C|GetPageArrow _returnvalue_4) (select _returnvalue_2 "(X=1.000000,Y=1.000000)" "(X=-1.000000,Y=1.000000)"))
      (Utilities|Array|Add (Variables|Default|GetWeaponPrice) (.Price (Utilities|Struct|BreakWeaponWidgetStructure _returnvalue_3)))
      (Utilities|Array|Add (Variables|Default|GetPageState) _output)
      (switch Utilities|FlowControl|Switch|SwitchonStates _output
        (:NewEnumerator0
          (Variables|/Script/UMG.TextBlock|SetText (Variables|/Game/Game/Widget/WBP_WeaponParent.WBP_WeaponParent_C|GetBUTTON _returnvalue_4) (|GenerictoText (Utilities|String|Append "ACHETER : 
" (Utilities|String|ToString(Integer) (.Price (Utilities|Struct|BreakWeaponWidgetStructure _returnvalue_3)))))))
        (:NewEnumerator1
          (Variables|/Script/UMG.TextBlock|SetText (Variables|/Game/Game/Widget/WBP_WeaponParent.WBP_WeaponParent_C|GetBUTTON _returnvalue_4) "ÉQUIPER ?"))
        (:NewEnumerator2
          (Variables|/Script/UMG.TextBlock|SetText (Variables|/Game/Game/Widget/WBP_WeaponParent.WBP_WeaponParent_C|GetBUTTON _returnvalue_4) "ÉQUIPÉE !"))))))

(fn UpdateWidgets
  (Utilities|Array|Clear (Variables|Default|GetWeaponPrice))
  (Utilities|Array|Clear (Variables|Default|GetPageState))
  (Utilities|Array|Clear (Variables|Default|GetPageTexture))
  (Utilities|Array|Clear (Variables|Default|GetPageClass))
  (for (_array_element _array_index) (Variables|Default|GetPageWeaponIndex)
    (CallFunction|CreateWeaponWidget _array_element)
    (UserInterface|SetWidget (Utilities|Array|Get(acopy) (Variables|Default|GetPageWidgets) _array_index) (Variables|Default|GetTempWidget))))