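; BP_Debris is a debris pickup actor that gets drawn into the player when the player enters its sphere trigger.
; On overlap with BP_Player, it records its start location and plays the Collect timeline, lerping toward the player's live position while shrinking from unit scale to zero.
; The graph only handles this visual pull: it neither destroys the actor nor grants anything, and the Damage event is empty.
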(event OnComponentBeginOverlap(Sphere)
  (params (OverlappedComponent :type Primitive%20Component%20Object%20Reference) (OtherActor :type Actor%20Object%20Reference) (OtherComp :type Primitive%20Component%20Object%20Reference) (OtherBodyIndex :type Integer) (bFromSweep :type Boolean) (SweepResult :type Hit%20Result%20Structure%20%28by%20ref%29))
  (bind _asbp_player (Utilities|Casting|CastToBP_Player OtherActor))
  (Variables|Default|SetStart (Transformation|GetActorLocation))
  (bind _alpha (Timeline|Collect Play)
    (:Update
      (Transformation|SetActorTransform (Math|Transform|MakeTransform (Math|Vector|Lerp(Vector) (Variables|Default|GetStart) (Transformation|GetActorLocation _asbp_player) _alpha) (Transformation|GetActorRotation) (Math|Vector|Lerp(Vector) "1.000000,1.000000,1.000000" "0, 0, 0" _alpha))))))

(event EventBeginPlay
  (|CallParentFunction) ; This node is disabled and will not be called.\nDrag off pins to build functionality.
)

(event Collision|EventActorBeginOverlap
  (params (OtherActor :type Actor%20Object%20Reference)))

(event EventTick
  (params (DeltaSeconds :type Float%20%28single-precision%29))
  (|CallParentFunction DeltaSeconds) ; This node is disabled and will not be called.\nDrag off pins to build functionality.
)

(event EventDamage
  (params (DamageValue :type Float%20%28double-precision%29)))

(fn ConstructionScript
  (|CallParentFunction))