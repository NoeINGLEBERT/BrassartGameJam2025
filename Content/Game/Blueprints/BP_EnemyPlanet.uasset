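; Enemy planet actor with random scale that drifts toward the world origin, carried sideways by its Velocity projected onto the tangent plane.
; On reaching the central sphere, debris snaps to the surface at small size, while other planets only print a death message.
; Debris shrinks as it approaches.
; At zero health it destroys itself, spawning a random number of SplitClass actors with randomized tangential velocities fanned evenly around the radial axis.
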(event Custom|HitPlanet
  (Variables|Default|SetHit true)
  (if (Variables|Default|GetIsDebris)
    (Transformation|SetWorldScale3D (Variables|Default|GetPlanet) "0.250000,0.250000,0.250000")
    (Transformation|SetActorLocation (* (Math|Vector|Normalize (Transformation|GetActorLocation)) (+ 2.5e+02 (* (.x (Variables|/Script/Engine.SceneComponent|GetRelativeScale3D (Variables|Default|GetPlanet))) 5e+01))) false false)
    (else
      (Development|PrintString "DEATH !!" true true "(R=1.000000,G=0.000000,B=0.000000,A=1.000000)"))))

(event EventTick
  (params (DeltaSeconds :type Float%20%28single-precision%29))
  (bind _returnvalue (Transformation|GetActorLocation))
  (bind _returnvalue_2 (Transformation|GetActorLocation))
  (bind _startlocation (Variables|Default|GetStartLocation))
  (bind _planet (Variables|Default|GetPlanet))
  (bind _planet_2 (Variables|Default|GetPlanet))
  (bind _scale (Variables|Default|GetScale))
  (bind _returnvalue_3 (Math|Vector|VectorLength _returnvalue_2))
  (bind _returnvalue_4 (Math|Vector|VectorLength _startlocation))
  (bind _relativescale3d (Variables|/Script/Engine.SceneComponent|GetRelativeScale3D _planet))
  (bind _relativescale3d_2 (Variables|/Script/Engine.SceneComponent|GetRelativeScale3D _planet_2))
  (bind _returnvalue_5 (* (.x _relativescale3d) 5e+01))
  (bind _returnvalue_6 (* (.x _relativescale3d_2) 5e+01))
  (bind _returnvalue_7 (Utilities|Operators|Subtract _returnvalue_3 _returnvalue_5 1e+03))
  (bind _returnvalue_8 (Utilities|Operators|Subtract _returnvalue_4 _returnvalue_6 1e+03))
  (bind _returnvalue_9 (/ _returnvalue_7 _returnvalue_8))
  (bind _returnvalue_10 (Math|Float|Power _returnvalue_9 0.75))
  (bind _returnvalue_11 (Math|Float|Lerp 0.25 _scale _returnvalue_10))
  (if (not (Variables|Default|GetHit))
    (Transformation|SetActorLocation (+ (Math|Vector|Lerp(Vector) _returnvalue "0, 0, 0" (* DeltaSeconds (Variables|Default|GetPlanetLinearSpeed))) (Math|Vector|ProjectVectorontoPlane (Variables|Default|GetVelocity) (Math|Vector|Normalize _returnvalue))) false false)
    (Utilities|FlowControl|Sequence
      (:then_0
        (if (<= (Utilities|Operators|Subtract (Math|Vector|VectorLength (Transformation|GetActorLocation)) (* (.x (Variables|/Script/Engine.SceneComponent|GetRelativeScale3D (Variables|Default|GetPlanet))) 5e+01) 2.5e+02) 0.0)
          (Utilities|FlowControl|DoOnce false
            (:Completed
              (CallFunction|HitPlanet)))))
      (:then_1
        (if (Variables|Default|GetIsDebris)
          (Transformation|SetWorldScale3D (Variables|Default|GetPlanet) (Math|Vector|MakeVector _returnvalue_11 _returnvalue_11 _returnvalue_11)))))))

(event EventBeginPlay
  (bind _asbp_player (Utilities|Casting|CastToBP_Player (Game|Player|GetPlayerPawn 0)))
  (Variables|Default|SetPlayer _asbp_player)
  (bind _output_get (Variables|Default|SetScale (Math|Random|RandomFloatinRange (Variables|Default|GetMinScale) (Variables|Default|GetMaxScale))))
  (Transformation|SetWorldScale3D (Variables|Default|GetPlanet) (Math|Vector|MakeVector _output_get _output_get _output_get))
  (Variables|Default|SetStartLocation (Transformation|GetActorLocation))
  (Variables|Default|SetSplitNumber (Math|Random|RandomIntegerinRange (Variables|Default|GetMinSplitNumber) (Variables|Default|GetMaxSplitNumber))))

(event EventDamage
  (params (DamageValue :type Float%20%28double-precision%29))
  (bind _splitnumber (Variables|Default|GetSplitNumber))
  (bind _splitforce (Variables|Default|GetSplitForce))
  (bind _output_get (Variables|Default|SetHealth (- (Variables|Default|GetHealth) DamageValue)))
  (if (<= _output_get 0.0)
    (Variables|Default|SetRandomVector (Math|Vector|Normalize (Math|Vector|ProjectVectorontoPlane (Math|Random|RandomUnitVector) (Math|Vector|Normalize (Transformation|GetActorLocation)))))
    (for _index (range 0 (- _splitnumber 1))
      (bind _returnvalue (Game|SpawnActorfromClass (Variables|Default|GetSplitClass) (Math|Transform|MakeTransform (Transformation|GetActorLocation) (Math|Random|RandomRotator true) "1.000000,1.000000,1.000000") "AlwaysSpawn" "MultiplyWithRoot" 0 0))
      (Variables|BP_EnemyPlanet_C|SetVelocity _returnvalue (* (Math|Random|RandomUnitVectorinConeinDegrees (Math|Vector|RotateVectorAroundAxis (Variables|Default|GetRandomVector) (* (/ 3.6e+02 (Math|Conversions|ToFloat(Integer) _splitnumber)) _index) (Math|Vector|Normalize (Transformation|GetActorLocation))) 45.0) (/ (Math|Random|RandomFloatinRange (* _splitforce 0.5) (* _splitforce 1.5)) 1e+01))))
    (Actor|DestroyActor)
    (else
      (Development|PrintString "OUCH !" true true "(R=1.000000,G=0.500000,B=0.000000,A=1.000000)"))))

(fn ConstructionScript)